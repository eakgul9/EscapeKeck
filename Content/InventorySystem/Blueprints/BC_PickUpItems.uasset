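; BC_PickUpItems is a data-driven world pickup that the player can inspect and collect into their inventory.
; The construction script loads ItemInfo from DT_PickUpItems by RowName and applies its mesh.
; Interact spawns a BC_Studio actor far out along X and sends it the player and item details for inspection.
; PickUp adds ItemInfo to the BP_TopDownCharacter's Inventory, then destroys the actor.
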(event EventPickUp
  ;[1 1 1] Pick Up Item
  (bind _asbp_top_down_character (Utilities|Casting|CastToBP_TopDownCharacter (Game|GetPlayerCharacter 0)))
  (Default|AddtoInventory (Variables|/Game/TopDown/Blueprints/BP_TopDownCharacter.BP_TopDownCharacter_C|GetInventory _asbp_top_down_character) (Variables|Default|GetItemInfo))
  (Actor|DestroyActor))

(event EventInteract
  (params (Player :type BP%20Top%20Down%20Character%20Object%20Reference))
  (bind _iteminfo (Variables|Default|GetItemInfo))
  ;[1 1 1] Item Interact
  (bind _returnvalue (Game|SpawnActorfromClass "/Game/InventorySystem/Blueprints/BC_Studio.BC_Studio_C" (Math|Transform|MakeTransform "1000000000.000000,0.000000,0.000000") "Undefined" "MultiplyWithRoot" 0 0))
  (Class|BIInteractInterface|InspectItem(Message) _returnvalue Player (Utilities|Struct|MakeF_ItemInfo (.name _iteminfo) (.icon _iteminfo) (.stackable _iteminfo) (.itemclass _iteminfo) (.description _iteminfo) 0 (.craftable _iteminfo) (.mesh _iteminfo) (.craftedname _iteminfo) (.numneededtocombine _iteminfo))))

(fn ConstructionScript
  (bind _returnvalue (Utilities|GetDataTableRow "/Game/InventorySystem/Blueprints/DT_PickUpItems.DT_PickUpItems" (Variables|Default|GetRowName))
    (:then
      (bind _output_get (Variables|Default|SetItemInfo _returnvalue))
      (Components|StaticMesh|SetStaticMesh (Variables|Default|GetMesh) (.mesh _output_get)))))