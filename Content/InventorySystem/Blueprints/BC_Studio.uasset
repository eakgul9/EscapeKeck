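; BC_Studio is an inspection studio actor that shows an inventory item's mesh for the player to rotate and zoom.
; InspectItem sets the mesh, opens WBP_InspectUI and moves input from the player to itself, disabling movement.
; Holding right mouse rotates the mesh with mouse axes, while the wheel zooms by changing the scene capture's clamped FOV.
; CloseInspect restores player control, removes the widget, ends inspection and destroys the actor.
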(event Input|EnhancedActionEvents|EnhancedInputActionRotateObject
  (params (ActionValue :type Boolean) (ElapsedSeconds :type Float%20%28double-precision%29) (TriggeredSeconds :type Float%20%28double-precision%29) (InputAction :type Input%20Action%20Object%20Reference :default "/Game/MechanicsInputs/Actions/RotateObject.RotateObject")))

(event Input|EnhancedActionEvents|EnhancedInputActionCloseInspect
  (params (ActionValue :type Boolean) (ElapsedSeconds :type Float%20%28double-precision%29) (TriggeredSeconds :type Float%20%28double-precision%29) (InputAction :type Input%20Action%20Object%20Reference :default "/Game/MechanicsInputs/Actions/CloseInspect.CloseInspect"))
  (bind _playercontroller (Variables|Default|GetPlayerController))
  ;[1 1 1] Exit
  (Input|DisableInput _playercontroller)
  (Input|EnableInput (Variables|Default|GetPlayer) _playercontroller)
  (Variables|/Game/TopDown/Blueprints/BP_TopDownController.BP_TopDownController_C|SetMovementDisabled _playercontroller false)
  (Widget|RemovefromParent (Variables|Default|GetInspectionWidget))
  (Variables|Default|SetInspectionWidget 0)
  (Default|EndInspection (Variables|Default|GetPlayer))
  (Actor|DestroyActor))

(event EventInspectItem
  (params (Player :type BP%20Top%20Down%20Character%20Object%20Reference) (ItemInfo :type F%20Item%20Info%20Structure))
  ;[1 1 1] Inspect Item
  (Variables|Default|SetPlayer Player)
  (Components|StaticMesh|SetStaticMesh (Variables|Default|GetItemToFocus) (.Mesh (Utilities|Struct|BreakF_ItemInfo ItemInfo)))
  (bind _returnvalue (UserInterface|CreateWidget "/Game/InventorySystem/Blueprints/WBP_InspectUI.WBP_InspectUI_C" 0 ItemInfo))
  (bind _output_get (Variables|Default|SetInspectionWidget _returnvalue))
  (UserInterface|Viewport|AddtoViewport _output_get 0)
  (bind _output_get_2 (Variables|Default|SetPlayerController (Variables|/Game/TopDown/Blueprints/BP_TopDownCharacter.BP_TopDownCharacter_C|GetPlayerController (Variables|Default|GetPlayer))))
  (Input|DisableInput (Variables|Default|GetPlayer) _output_get_2)
  (Variables|/Game/TopDown/Blueprints/BP_TopDownController.BP_TopDownController_C|SetMovementDisabled (Variables|/Game/TopDown/Blueprints/BP_TopDownCharacter.BP_TopDownCharacter_C|GetPlayerController (Variables|Default|GetPlayer)) true)
  (Input|EnableInput _output_get_2))

(event Input|MouseEvents|MouseX
  (params (AxisValue :type Float%20%28single-precision%29))
  ;[1 1 1] X-axis Rotation
  (if (Variables|Default|GetCanRotate)
    (Transformation|SetWorldRotation (Variables|Default|GetItemToFocus) (Math|Rotator|CombineRotators (Transformation|GetWorldRotation (Variables|Default|GetItemToFocus)) (Math|Rotator|MakeRotator 0.0 0.0 (* AxisValue -2.0))) false false)))

(event Input|MouseEvents|MouseY
  (params (AxisValue :type Float%20%28single-precision%29))
  ;[1 1 1] Y-axis Rotation
  (if (Variables|Default|GetCanRotate)
    (Transformation|SetWorldRotation (Variables|Default|GetItemToFocus) (Math|Rotator|CombineRotators (Transformation|GetWorldRotation (Variables|Default|GetItemToFocus)) (Math|Rotator|MakeRotator 0.0 (* AxisValue -2.0) 0.0)) false false)))

(event Input|MouseEvents|MouseWheelUp
  (params (Key :type Key%20Structure :default "None"))
  (bind _scenecapturecomponent2d (Variables|Default|GetSceneCaptureComponent2D))
  ;[1 1 1] Zoom in
  (:Pressed
    (Variables|/Script/Engine.SceneCaptureComponent2D|SetFOVAngle _scenecapturecomponent2d (Math|Float|Clamp(Float) (- (Variables|/Script/Engine.SceneCaptureComponent2D|GetFOVAngle _scenecapturecomponent2d) (Variables|Default|GetZoomSpeed)) 47.0 105.0))))

(event Input|MouseEvents|RightMouseButton
  (params (Key :type Key%20Structure :default "None"))
  ;[1 1 1] Enable Rotation
  (:Pressed
    (Variables|Default|SetCanRotate true))
  (:Released
    (Variables|Default|SetCanRotate false)))

(event Input|MouseEvents|MouseWheelDown
  (params (Key :type Key%20Structure :default "None"))
  (bind _scenecapturecomponent2d (Variables|Default|GetSceneCaptureComponent2D))
  ;[1 1 1] Zoom out
  (:Pressed
    (Variables|/Script/Engine.SceneCaptureComponent2D|SetFOVAngle _scenecapturecomponent2d (Math|Float|Clamp(Float) (+ (Variables|/Script/Engine.SceneCaptureComponent2D|GetFOVAngle _scenecapturecomponent2d) (Variables|Default|GetZoomSpeed)) 47.0 105.0))))

(fn ConstructionScript)