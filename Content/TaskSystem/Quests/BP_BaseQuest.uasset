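; BP_BaseQuest is the base class for quests in the task system, holding a root objective collection.
; On BeginPlay it constructs the root collection, populates it with objectives, then activates it.
; The construct and populate functions are placeholders that print red error messages, so child quests are expected to override them.
; A getter exposes the root collection.
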(event EventBeginPlay
  ;[1 1 1] Populates objectives and activates root objective
  (bind _rootobjcollection (Private|ConstructRootObjectiveCollection))
  (bind _output_get (Variables|Private|SetRootObjectiveCollection _rootobjcollection))
  (Private|PopulateObjectives _output_get)
  (Default|ActivateObjective (Variables|Private|GetRootObjectiveCollection)))

(fn ConstructionScript)

(fn ConstructRootObjectiveCollection
  (Development|PrintString "Error: Create Root Objective Collection called for root class!!" true true "(R=1.000000,G=0.000000,B=0.008303,A=1.000000)")
  (return 0))

(fn PopulateObjectives
  (params (RootObjCollection :type BP%20Objective%20Collection%20Object%20Reference))
  (Development|PrintString "Error: Populate Objectives called for root class!!" true true "(R=1.000000,G=0.005876,B=0.000000,A=1.000000)"))

(fn GetRootObjCollection
  (return (Variables|Private|GetRootObjectiveCollection)))