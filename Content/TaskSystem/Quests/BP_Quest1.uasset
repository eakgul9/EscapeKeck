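; BP_Quest1 is a quest that defines an "Explore Keck Lab" task with an objective to visit the tea station.
; ConstructRootObjectiveCollection creates the root objective collection with ordered completion required.
; PopulateObjectives adds a single reach-destination objective to that collection, targeting PointATrigger.
; The event graph holds no active logic, so the Blueprint only supplies the quest's objective structure.
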(event EventBeginPlay
  (|CallParentFunction) ; This node is disabled and will not be called.\nDrag off pins to build functionality.
)

(event Collision|EventActorBeginOverlap
  (params (OtherActor :type Actor%20Object%20Reference)))

(event EventTick
  (params (DeltaSeconds :type Float%20%28single-precision%29)))

(event EventOnBecomeViewTarget
  (params (PC :type Player%20Controller%20Object%20Reference)))

(fn ConstructionScript
  (|CallParentFunction))

(fn ConstructRootObjectiveCollection
  (bind _returnvalue (Game|ConstructObjectfromClass self "/Game/TaskSystem/Objectives/BP_ObjectiveCollection.BP_ObjectiveCollection_C" true "Explore Keck Lab"))
  (return _returnvalue))

(fn PopulateObjectives
  (params (RootObjCollection :type BP%20Objective%20Collection%20Object%20Reference))
  (bind _returnvalue (Game|ConstructObjectfromClass self "/Game/TaskSystem/Objectives/BP_ObjectiveReachDestination.BP_ObjectiveReachDestination_C" (Variables|Default|GetPoint%20A%20Trigger) "Visit the Tea Station"))
  (Default|AddObjective RootObjCollection _returnvalue))