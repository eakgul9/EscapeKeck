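; BP_ObjectiveReachDestination is a task system objective that completes when the player character reaches a destination actor.
; On activation it runs the parent logic and binds to the Destination's begin overlap event.
; An overlap by a BP_TopDownCharacter unbinds the event, sets the ReachedDestination flag and fires the completion dispatcher with itself.
; GetIsComplete reports that flag.
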(event Custom|OnActorBeginOverlap_Event
  (params (OverlappedActor :type Actor%20Object%20Reference) (OtherActor :type Actor%20Object%20Reference))
  (Utilities|Casting|CastToBP_TopDownCharacter OtherActor)
  (Collision|UnbindEventfromOnActorBeginOverlap (Variables|Default|GetDestination) (delegate Custom|OnActorBeginOverlap_Event))
  (Variables|Default|SetReachedDestination true)
  (Default|CallOnCompleted self))

(event EventActivateObjective
  (|CallParentFunction)
  (EventDispatchers|AssignOnActorBeginOverlap (Variables|Default|GetDestination) (delegate Custom|OnActorBeginOverlap_Event)))

(fn GetIsComplete
  (return (Variables|Default|GetReachedDestination)))